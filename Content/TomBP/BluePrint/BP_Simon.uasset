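; BP_Simon runs a multi-level Simon memory game, started when a player overlaps its box.
; Each level builds a random sequence of stand indices from its settings, plays it through the Stands, then checks player notes against it.
; Mistakes restart the level, successes advance it, and the final win triggers confetti and a timeline.
; The construction script caps note counts to the stand count for levels without duplicates.
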(event `self.ReceiveBeginPlay`
  (for _array_element (`self.Stands`)
    (`/Engine/EditorBlueprintResources/StandardMacros.IsValid` _array_element
      (:`Is Valid`
        (set `/Game/TomBP/BluePrint/BP_Stand.SimonMain_Ref` self _array_element)))))

(event `AddAnotherNote`
  (bind (_numberofnotes _timebetweennotes _canduplicatenotes) (break `/Game/TomBP/BluePrint/SimonLevel_Struct` (`|GetArrayItem` (`self.LevelSettings`) (`self.CurrentLevel`))))
  ; Creer une sequence random basé sur les parametres du level
  (if (> (`KismetArrayLibrary.Array_Length` (`self.Stands`)) 0) :!label _label
    (if _canduplicatenotes
      (`KismetArrayLibrary.Array_Add` (`self.SimonSequence`) (`KismetMathLibrary.RandomIntegerInRange` 0 (`KismetArrayLibrary.Array_LastIndex` (`self.Stands`))))
      (else
        (`KismetArrayLibrary.Array_AddUnique` (`self.SimonSequence`) (`KismetMathLibrary.RandomIntegerInRange` 0 (`KismetArrayLibrary.Array_LastIndex` (`self.Stands`))))))
    (if (< (`KismetArrayLibrary.Array_Length` (`self.SimonSequence`)) _numberofnotes)
      (`KismetSystemLibrary.Delay` 0.0)
      (`self.AddAnotherNote`)
      (else
        (`KismetSystemLibrary.Delay` 1.0)
        (`self.PlaySimonSequence`)))))

(event `self.Box.OnComponentBeginOverlap`
  (params (OverlappedComponent :type "PrimitiveComponent Object Reference") (OtherActor :type "Actor Object Reference") (OtherComp :type "PrimitiveComponent Object Reference") (OtherBodyIndex :type Integer) (bFromSweep :type Boolean) (SweepResult :type "HitResult Structure (by ref)"))
  ; Overlap Event, Start Level
  (if (and (`KismetSystemLibrary.DoesImplementInterface` OtherActor "/Game/TomBP/BluePrint/Interface/BPI_Player.BPI_Player_C") (not (`self.isPlaying`)))
    (set `self.isPlaying` true)
    (`self.StartLevel`)))

(event `CreateSimonSequence`
  ; Creer une sequence random basé sur les parametres du level
  (`KismetArrayLibrary.Array_Clear` (`self.SimonSequence`))
  (goto _label))

(event `StartLevel`
  ; Start New Level
  (`KismetArrayLibrary.Array_Clear` (`self.PlayerSequence`))
  (set `self.CurrentNote` 0)
  (set `self.isPlayersTurn` false)
  (`self.CreateSimonSequence`))

(event `PlaySimonSequence`
  (`/Game/TomBP/BluePrint/BP_Stand.PlayNote` (`|GetArrayItem` (`self.Stands`) (`|GetArrayItem` (`self.SimonSequence`) (`self.CurrentNote`))))
  (`KismetSystemLibrary.Delay` (`.TimeBetweenNotes_9_68F9D4AE4B8CE6578F64C396C5DA9614` (break `/Game/TomBP/BluePrint/SimonLevel_Struct` (`|GetArrayItem` (`self.LevelSettings`) (`self.CurrentLevel`)))))
  (`/Engine/EditorBlueprintResources/StandardMacros.IncrementInt` (`self.CurrentNote`)
    (:`  `
      (if (< (`self.CurrentNote`) (`KismetArrayLibrary.Array_Length` (`self.SimonSequence`)))
        (`self.PlaySimonSequence`)
        (else
          (set `self.isPlayersTurn` true))))))

(event `PlayerPlayedNote`
  (params (Note :type Integer))
  (set `self.isPlayersTurn` false)
  (bind _returnvalue (`KismetArrayLibrary.Array_Add` (`self.PlayerSequence`) Note))
  (if (== Note (`|GetArrayItem` (`self.SimonSequence`) _returnvalue))
    (`/Game/TomBP/BluePrint/BP_Stand.PlayNote` (`|GetArrayItem` (`self.Stands`) Note))
    (if (>= (`KismetArrayLibrary.Array_Length` (`self.PlayerSequence`)) (`KismetArrayLibrary.Array_Length` (`self.SimonSequence`)))
      (if (< (`self.CurrentLevel`) (`KismetArrayLibrary.Array_LastIndex` (`self.LevelSettings`)))
        (`/Engine/EditorBlueprintResources/StandardMacros.IncrementInt` (`self.CurrentLevel`)
          (:`  `
            (`GameplayStatics.PlaySound2D` "/Game/TomBP/Sounds/Win_Cue.Win_Cue" 1.0 1.0 0.0 null null)
            (`KismetSystemLibrary.Delay` 2.0)
            (`self.StartLevel`)))
        (else
          (`KismetSystemLibrary.Delay` 2.0)
          (`GameplayStatics.PlaySound2D` "/Game/TomBP/Sounds/WinAll_Cue.WinAll_Cue" 1.0 1.0 0.0 null null)
          (`KismetSystemLibrary.Delay` 3.0)
          ;[1 0 0 0.5] ICI POUR METTRE L4EXPLOSION
          (`ActorComponent.Activate` (`self.NS_Confeti`) false)
          (`KismetSystemLibrary.Delay` 1.0)
          (`ActorComponent.Activate` (`self.NS_Confeti`) false)
          (`KismetSystemLibrary.Delay` 1.0)
          (`ActorComponent.Deactivate` (`self.NS_Confeti`))
          (`Timeline|Timeline`)))
      (else
        (set `self.isPlayersTurn` true)))
    (else
      (for _array_element (`self.Stands`)
        (`/Game/TomBP/BluePrint/BP_Stand.PlayError` _array_element))
      (`KismetSystemLibrary.Delay` 0.2)
      (`self.StartLevel`))))

(fn `UserConstructionScript`
  (bind _returnvalue (`KismetArrayLibrary.Array_Length` (`self.Stands`)))
  (for (_array_element _array_index) (`self.LevelSettings`)
    (bind ((`NumberOfNotes_12_761F0C2E4DF892B9277063ADD379E0AA` _numberofnotes) (`CanDuplicateNotes_11_8BCC2FF14B8061B2D0C10D90CD04FC6E` _canduplicatenotes)) (break `/Game/TomBP/BluePrint/SimonLevel_Struct` _array_element))
    (if _canduplicatenotes
      _
      (elif (> _numberofnotes _returnvalue)
        (bind _structout (setmembers `/Game/TomBP/BluePrint/SimonLevel_Struct` :`StructRef` _array_element :`NumberOfNotes` _returnvalue))
        (`KismetArrayLibrary.Array_Set` (`self.LevelSettings`) _array_index _structout)))))