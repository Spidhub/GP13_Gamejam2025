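; BP_Base is a Blueprint that slides a mesh along a timeline when an event bound through SimonRef fires.
; On BeginPlay it passes its StartTimeline event to SimonRef's BindEventToTimeline, and that event plays the timeline from the start.
; Each update lerps StaticMesh's relative location from the local origin to StaticMesh1's relative location, so the second mesh's placement defines the destination.
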(event `Timeline`
  (bind (_direction _newtrack_1) (`Timeline|Timeline_0` :!via `PlayFromStart`)
    (:`Update`
      (`SceneComponent.K2_SetRelativeLocation` (`self.StaticMesh`) (`KismetMathLibrary.VLerp` (0.0 0.0 0.0) (`SceneComponent.RelativeLocation` (`self.StaticMesh1`)) _newtrack_1) false false))))

(event `self.ReceiveBeginPlay`
  (add `/Game/TomBP/BluePrint/BP_Simon.Timeline` (`self.SimonRef`) (delegate `StartTimeline`)))

(event `StartTimeline`
  (`self.Timeline`))

(fn `UserConstructionScript`)