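; BP_MusicMaster is a music manager that switches between two zone tracks, Crazyspace and SubdreamSpace_Philately.
; On BeginPlay it creates a 2D sound for each track and stores them as SonZone1 and SonZone2.
; The SoundTrigger event takes a song index, stops the other track and plays the selected one from the start, with no crossfade.
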(event `self.ReceiveBeginPlay`
  (bind _returnvalue (`GameplayStatics.CreateSound2D` "/Game/TomBP/Sounds/crazy-space.crazy-space" 1.0 1.0 0.0 null))
  (set `self.SonZone1` _returnvalue)
  (bind _returnvalue_2 (`GameplayStatics.CreateSound2D` "/Game/TomBP/Sounds/Subdream-Space_Philately.Subdream-Space_Philately" 1.0 1.0 0.0 null))
  (set `self.SonZone2` _returnvalue_2))

(event `SoundTrigger`
  (params (`Song?` :type Integer))
  (switch `int` `Song?`
    (:`0`
      (`AudioComponent.Stop` (`self.SonZone2`))
      (`AudioComponent.Play` (`self.SonZone1`) 0.0))
    (:`1`
      (`AudioComponent.Stop` (`self.SonZone1`))
      (`AudioComponent.Play` (`self.SonZone2`) 0.0))))

(fn `UserConstructionScript`)