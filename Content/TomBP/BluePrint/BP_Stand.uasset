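; BP_Stand is one colored note pad in a Simon-style memory game.
; On player interaction during their turn, it reports its index to SimonMainRef; look-at briefly applies an overlay, though that turn check is flagged as not working.
; PlayNote and PlayError pair sound with timed glow on a dynamic material colored at construction.
; A timeline, started through an event bound on SimonRef, destroys the stand.
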(event `Timeline`
  (`self.K2_DestroyActor`))

(event `self.ReceiveBeginPlay`
  (`AudioComponent.SetSound` (`self.Audio`) (`self.Sound`))
  (add `/Game/TomBP/BluePrint/BP_Simon.Timeline` (`self.SimonRef`) (delegate `StartTimeline`)))

(event `StartTimeline`
  (`self.Timeline`))

(event `/Game/TomBP/BluePrint/Interface/BPI_Interact.OnInteract`
  (params (Actor :type "Actor Object Reference"))
  (if (`KismetSystemLibrary.DoesImplementInterface` Actor "/Game/TomBP/BluePrint/Interface/BPI_Player.BPI_Player_C")
    (bind _simonmain_ref (`self.SimonMain_Ref`)
      (:`then`
        (if (`/Game/TomBP/BluePrint/BP_Simon.isPlayersTurn` _simonmain_ref)
          (`/Game/TomBP/BluePrint/BP_Simon.PlayerPlayedNote` (`self.SimonMain_Ref`) (`self.Index`))))
      (:`else`))))

(event `PlayNote`
  (`AudioComponent.Play` (`self.Audio`) 0.0)
  (`MaterialInstanceDynamic.SetScalarParameterValue` (`self.DynMat`) "Intensity" 10.0)
  (`KismetSystemLibrary.Delay` 0.85)
  (`AudioComponent.Stop` (`self.Audio`))
  (`MaterialInstanceDynamic.SetScalarParameterValue` (`self.DynMat`) "Intensity" 0.0))

(event `/Game/TomBP/BluePrint/Interface/BPI_Interact.OnLookAt`
  (params (Actor :type "Actor Object Reference"))
  (bind _simonmain_ref (`self.SimonMain_Ref`)
    (:`then`
      ;[1 0.1932 0 0.5] Ne fonctionne pas...
      (if (`/Game/TomBP/BluePrint/BP_Simon.isPlayersTurn` _simonmain_ref)
        (`MeshComponent.SetOverlayMaterial` (`self.Capsule`) "/Game/TomBP/Materials/M_Overlay.M_Overlay")
        (`KismetSystemLibrary.RetriggerableDelay` 0.11)
        (`MeshComponent.SetOverlayMaterial` (`self.Capsule`) null)))
    (:`else`)))

(event `PlayError`
  (`GameplayStatics.PlaySound2D` "/Game/TomBP/Sounds/Loose_Cue.Loose_Cue" 1.0 1.0 0.0 null null)
  (`MaterialInstanceDynamic.SetVectorParameterValue` (`self.DynMat`) "Color" (struct :`R` 1.0 :`B` 0.018539 :`A` 1.0))
  (`MaterialInstanceDynamic.SetScalarParameterValue` (`self.DynMat`) "Intensity" 10.0)
  (`KismetSystemLibrary.Delay` 1.0)
  (`MaterialInstanceDynamic.SetScalarParameterValue` (`self.DynMat`) "Intensity" 0.0)
  (`MaterialInstanceDynamic.SetVectorParameterValue` (`self.DynMat`) "Color" (`self.Color`)))

(fn `UserConstructionScript`
  (bind _returnvalue (`PrimitiveComponent.CreateDynamicMaterialInstance` (`self.Capsule`) 0 "/Game/TomBP/Materials/M_Color.M_Color" "None"))
  (bind _output_get (set `self.DynMat` _returnvalue))
  (`MaterialInstanceDynamic.SetVectorParameterValue` _output_get "Color" (`self.Color`)))