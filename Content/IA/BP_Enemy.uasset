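; Enemy character Blueprint that takes damage, can shoot and ragdolls when its health runs out.
; AnyDamage subtracts from Health while it is positive, then enables physics simulation, full blend weight and collision on the Mesh at zero or below.
; Fire line-traces from WeaponMuzzle along the FollowCamera forward vector, with debug drawing, and applies fixed damage to the hit actor.
; UpdateWalkSpeed sets the movement component's max walk speed.
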(event `self.ReceiveAnyDamage`
  (params (Damage :type "Float (single-precision)") (DamageType :type "DamageType Object Reference") (InstigatedBy :type "Controller Object Reference") (DamageCauser :type "Actor Object Reference"))
  (bind _mesh (`self.Mesh`))
  (bind _health (`self.Health`))
  (if (> _health 0.0)
    (set `self.Health` (- _health Damage))
    (if (<= (`self.Health`) 0.0)
      (`PrimitiveComponent.SetSimulatePhysics` _mesh true)
      (`SkeletalMeshComponent.SetPhysicsBlendWeight` _mesh 1.0)
      (`PrimitiveComponent.SetCollisionEnabled` _mesh "QueryAndPhysics"))))

(fn `Fire`
  (bind (_returnvalue_location _returnvalue_rotation) (`KismetMathLibrary.BreakTransform` (`SceneComponent.K2_GetComponentToWorld` (`self.FollowCamera`))))
  (bind _returnvalue_location_2 (`KismetMathLibrary.BreakTransform` (`SceneComponent.K2_GetComponentToWorld` (`self.WeaponMuzzle`))))
  (bind (_outhit _returnvalue) (`KismetSystemLibrary.LineTraceSingle` :`Start` _returnvalue_location_2 :`End` (+ _returnvalue_location_2 (* (`KismetMathLibrary.GetForwardVector` _returnvalue_rotation) 1500.0)) :`TraceChannel` "TraceTypeQuery3" :`DrawDebugType` "ForDuration"))
  (if _returnvalue
    (`GameplayStatics.ApplyDamage` (`.HitActor` (`GameplayStatics.BreakHitResult` _outhit)) 20.0)))

(fn `UpdateWalkSpeed`
  (params (NewWalkSpeed :type "Float (double-precision)"))
  (set `CharacterMovementComponent.MaxWalkSpeed` NewWalkSpeed (`self.CharacterMovement`)))

(fn `UserConstructionScript`)