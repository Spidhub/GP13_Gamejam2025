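; BP_Boss is a boss enemy that shoots at the player and notifies the game instance when it dies.
; Fire runs a debug-drawn line trace from the weapon muzzle to player 0, damaging whatever it hits; the cooldown resets only after a hit.
; AnyDamage reduces health, then on death enables mesh ragdoll physics and, after a delay, calls BossDead and destroys the actor.
; UpdateWalkSpeed sets movement speed.
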(event `self.ReceiveBeginPlay`
  (bind _asbp_gameinstance (cast `/Game/BP_Gameinstance` (`GameplayStatics.GetGameInstance`)))
  (set `self.As BP Gameinstance` _asbp_gameinstance))

(event `self.ReceiveAnyDamage`
  (params (Damage :type "Float (single-precision)") (DamageType :type "DamageType Object Reference") (InstigatedBy :type "Controller Object Reference") (DamageCauser :type "Actor Object Reference"))
  (bind _mesh (`self.Mesh`))
  (bind _health (`self.Health`))
  (if (> _health 0.0)
    (set `self.Health` (- _health Damage))
    (if (<= (`self.Health`) 0.0)
      (`PrimitiveComponent.SetSimulatePhysics` _mesh true)
      (`SkeletalMeshComponent.SetPhysicsBlendWeight` _mesh 1.0)
      (`PrimitiveComponent.SetCollisionEnabled` _mesh "QueryAndPhysics")
      (set `self.Alive?` false)
      (`KismetSystemLibrary.Delay` 5.0)
      (`/Game/BP_Gameinstance.BossDead` (`self.As BP Gameinstance`))
      (`self.K2_DestroyActor`))))

(event `Fire`
  (bind _returnvalue_location (`KismetMathLibrary.BreakTransform` (`self.GetTransform` (`GameplayStatics.GetPlayerPawn` 0))))
  (bind _returnvalue_location_2 (`KismetMathLibrary.BreakTransform` (`SceneComponent.K2_GetComponentToWorld` (`self.WeaponMuzzle`))))
  (if (`self.Alive?`)
    (if (not (`self.OnCD?`))
      (set `self.OnCD?` true)
      (bind (_outhit _returnvalue) (`KismetSystemLibrary.LineTraceSingle` :`Start` _returnvalue_location_2 :`End` _returnvalue_location :`TraceChannel` "TraceTypeQuery3" :`DrawDebugType` "ForDuration"))
      (if _returnvalue
        (`GameplayStatics.ApplyDamage` (`.HitActor` (`GameplayStatics.BreakHitResult` _outhit)) 20.0)
        (`KismetSystemLibrary.Delay` 0.5)
        (set `self.OnCD?` false)))))

(fn `UpdateWalkSpeed`
  (params (NewWalkSpeed :type "Float (double-precision)"))
  (set `CharacterMovementComponent.MaxWalkSpeed` NewWalkSpeed (`self.CharacterMovement`)))

(fn `UserConstructionScript`)