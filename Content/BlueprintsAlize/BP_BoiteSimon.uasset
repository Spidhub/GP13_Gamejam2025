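; Simon box actor that slides its box mesh when the referenced Simon actor triggers it.
; On BeginPlay it passes StartTimeline to SimonRef through BindEventToTimeline.
; That event plays a timeline that lerps SMBoiTeSimon's relative location from the origin to that of SMBoiTeSimon1, which serves as the end-position marker.
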(event `Timeline1`
  (bind (_direction _newtrack_1) (`Timeline|Timeline`)
    (:`Update`
      (`SceneComponent.K2_SetRelativeLocation` (`self.SM_BoiTeSimon`) (`KismetMathLibrary.VLerp` (0.0 0.0 0.0) (`SceneComponent.RelativeLocation` (`self.SM_BoiTeSimon1`)) _newtrack_1) false false))))

(event `self.ReceiveBeginPlay`
  (add `/Game/TomBP/BluePrint/BP_Simon.Timeline` (`self.SimonRef`) (delegate `StartTimeline`)))

(event `StartTimeline`
  (`self.Timeline1`))

(fn `UserConstructionScript`)